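; Passive hero gameplay ability that grants stacks of an armor gameplay effect over time and loses one stack each time damage is received.
; On activation, a looping WaitDelay task applies a stack after each recharge delay, while a WaitReceiveDamage task removes stacks by granted tag.
; A stack-change listener, started once the effect handle exists, stops the loop at max stacks and restarts it when the count drops from max.
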(event Custom|StackChange
  (bind _max_stacks (Variables|Default|GetMax%20Stacks))
  ;[1 1 1] Add a stack every X seconds
  (Utilities|FlowControl|DoOnce false
    (:Completed
      (bind (_asynctaskproxy _handle _newcount _oldcount) (|WaitforGameplayEffectStackChange (Variables|Default|GetGE_StackGeneratorHandle))
        (:then
          (Variables|Default|SetWaitStackChangeTask _asynctaskproxy))
        (:OnChange
          (if (== _newcount _max_stacks)
            (bind _waitdelaytask (Variables|Default|GetWaitDelayTask)
              (:then
                (GameplayTasks|EndTask _waitdelaytask)
                (Variables|Default|SetShouldLoopWaitDelayTask false))
              (:else))
            (elif (== _oldcount _max_stacks)
              (bind _asynctaskproxy_2 (Ability|Tasks|WaitDelay (Variables|Default|GetRechargeDelay) :!label _label)
                (:then
                  (Variables|Default|SetWaitDelayTask _asynctaskproxy_2)
                  (Variables|Default|SetShouldLoopWaitDelayTask true)
                  (Utilities|FlowControl|DoOnce false
                    (:Completed
                      ;[1 1 1] Remove a stack when we receive damage
                      (bind _asynctaskproxy_3 (|WaitReceiveDamage false)
                        (:then
                          (Variables|Default|SetWaitReceiveDamageTask _asynctaskproxy_3))
                        (:OnDamage
                          (Ability|RemoveGameplayEffectFromOwnerWithGrantedTags "(GameplayTags=((TagName=\"Effect.Hero.PassiveArmor\")))" 1))))))
                (:OnFinish
                  (bind _returnvalue (Ability|ApplyGameplayEffectToOwner (Variables|Default|GetGEArmorClass) (Ability|GetAbilityLevel)))
                  (Variables|Default|SetGE_StackGeneratorHandle _returnvalue)
                  (CallFunction|StackChange) ; Need the GE Handle to exist so we start this here
                  (if (Variables|Default|GetShouldLoopWaitDelayTask)
                    (goto _label)))))))))))

(event Ability|EventActivateAbility
  ;[1 1 1] Add a stack every X seconds
  (bind _asynctaskproxy (Ability|Tasks|WaitDelay (Variables|Default|GetRechargeDelay) :!label _label)
    (:then
      (Variables|Default|SetWaitDelayTask _asynctaskproxy)
      (Variables|Default|SetShouldLoopWaitDelayTask true)
      (Utilities|FlowControl|DoOnce false
        (:Completed
          ;[1 1 1] Remove a stack when we receive damage
          (bind _asynctaskproxy_2 (|WaitReceiveDamage false)
            (:then
              (Variables|Default|SetWaitReceiveDamageTask _asynctaskproxy_2))
            (:OnDamage
              (Ability|RemoveGameplayEffectFromOwnerWithGrantedTags "(GameplayTags=((TagName=\"Effect.Hero.PassiveArmor\")))" 1))))))
    (:OnFinish
      (bind _returnvalue (Ability|ApplyGameplayEffectToOwner (Variables|Default|GetGEArmorClass) (Ability|GetAbilityLevel)))
      (Variables|Default|SetGE_StackGeneratorHandle _returnvalue)
      (CallFunction|StackChange) ; Need the GE Handle to exist so we start this here
      (if (Variables|Default|GetShouldLoopWaitDelayTask)
        (goto _label)))))

(event Ability|EventOnEndAbility
  (params (bWasCancelled :type Boolean))
  (bind _waitstackchangetask (Variables|Default|GetWaitStackChangeTask)
    (:then
      (GameplayTasks|EndTask _waitstackchangetask))
    (:else
      _))
  (bind _waitdelaytask (Variables|Default|GetWaitDelayTask)
    (:then
      (GameplayTasks|EndTask _waitdelaytask))
    (:else
      _))
  (bind _waitreceivedamagetask (Variables|Default|GetWaitReceiveDamageTask)
    (:then
      (GameplayTasks|EndTask _waitreceivedamagetask))
    (:else)))