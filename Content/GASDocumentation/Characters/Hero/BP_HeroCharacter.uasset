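; Hero character Blueprint for the GASDocumentation project, adding a debug printout of Gameplay Ability System attributes.
; On possession it calls the parent, then a Test event waits one tick and prints the name of every attribute on its Ability System Component.
; BeginPlay only calls the parent, and Tick, overlap and the construction script add no logic.
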(event Custom|Test
  (Utilities|FlowControl|DelayUntilNextTick)
  (Utilities|FlowControl|Sequence
    (:then_0
      (for _array_element (Class|AbilitySystemComponent|GetAllAttributes (Ability|GetAbilitySystemComponent 0))
        (Development|PrintString (Utilities|Struct|BreakGameplayAttribute _array_element))))))

(event EventBeginPlay
  (|CallParentFunction))

(event Collision|EventActorBeginOverlap
  (params (OtherActor :type Actor%20Object%20Reference)))

(event EventTick
  (params (DeltaSeconds :type Float%20%28single-precision%29)))

(event EventPossessed
  (params (NewController :type Controller%20Object%20Reference))
  (|CallParentFunction NewController)
  (CallFunction|Test))

(fn ConstructionScript)